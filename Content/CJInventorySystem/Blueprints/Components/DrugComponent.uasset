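; Drug component for an inventory system that maintains an on-screen pickup list of drug items.
; AddDrugItem looks up a DrugList data table row, creates the container widget on first use, appends a slot with icon, name and description to its grid, and shows the mouse cursor.
; RemoveDrugItem drops slots matched by display name, rebuilds the single-column grid, and closes the container and hides the cursor once empty.
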(fn `AddDrugItem`
  (params (DrugActorName :type Name))
  ;[1 1 1] 添加药品到拾取列表
  (bind _returnvalue (`|GetDataTableRow` "/Game/CJInventorySystem/Items/DrugList.DrugList" DrugActorName)
    (:`then`
      (if (not (`self.IsCreateContainer`))
        (bind _returnvalue_2 (`|CreateWidget` "/Game/CJInventorySystem/UI/Blueprints/Inventory/Container.Container_C"))
        (bind _output_get (set `self.Container` _returnvalue_2))
        (`UserWidget.AddToViewport` _output_get 0)
        (set `self.IsCreateContainer` true))
      (bind _returnvalue_3 (`|CreateWidget` "/Game/CJInventorySystem/UI/Blueprints/Inventory/ContainerSlot.ContainerSlot_C"))
      (bind (_icon _name _description) (break `/Game/CJInventorySystem/Blueprints/Inventory/DrugInfo` _returnvalue))
      (set `/Game/CJInventorySystem/UI/Blueprints/Inventory/ContainerSlot.IconValue` _icon _returnvalue_3)
      (set `/Game/CJInventorySystem/UI/Blueprints/Inventory/ContainerSlot.NameValue` (`KismetTextLibrary.Conv_NameToText` _name) _returnvalue_3)
      (set `/Game/CJInventorySystem/UI/Blueprints/Inventory/ContainerSlot.DescriptionValue` (`KismetTextLibrary.Conv_StringToText` _description) _returnvalue_3)
      (bind _returnvalue_4 (`KismetArrayLibrary.Array_Add` (`/Game/CJInventorySystem/UI/Blueprints/Inventory/Container.ContainerSlots` (`self.Container`)) _returnvalue_3))
      (bind _returnvalue_5 (`PanelWidget.AddChild` (`/Game/CJInventorySystem/UI/Blueprints/Inventory/Container.ContainerGridPanel` (`self.Container`)) _returnvalue_3))
      (bind _asuniform_grid_slot (cast `UniformGridSlot` _returnvalue_5))
      (`UniformGridSlot.SetRow` _asuniform_grid_slot _returnvalue_4)
      (`UniformGridSlot.SetColumn` _asuniform_grid_slot 0)
      (if (not (`self.IsShowMouseCursor`))
        (set `PlayerController.bShowMouseCursor` true (`GameplayStatics.GetPlayerController` 0))
        (set `self.IsShowMouseCursor` true)))))

(fn `RebuildContainer`
  ;[1 1 1] 重新构建拾取列表
  (`PanelWidget.ClearChildren` (`/Game/CJInventorySystem/UI/Blueprints/Inventory/Container.ContainerGridPanel` (`self.Container`)))
  (for (_array_element _array_index) (`/Game/CJInventorySystem/UI/Blueprints/Inventory/Container.ContainerSlots` (`self.Container`))
    (bind _returnvalue (`PanelWidget.AddChild` (`/Game/CJInventorySystem/UI/Blueprints/Inventory/Container.ContainerGridPanel` (`self.Container`)) _array_element))
    (bind _asuniform_grid_slot (cast `UniformGridSlot` _returnvalue))
    (`UniformGridSlot.SetRow` _asuniform_grid_slot _array_index)
    (`UniformGridSlot.SetColumn` _asuniform_grid_slot 0)))

(fn `RemoveDrugItem`
  (params (DrugName :type Name))
  (bind _containerslots (`/Game/CJInventorySystem/UI/Blueprints/Inventory/Container.ContainerSlots` (`self.Container`)))
  ;[1 1 1] 移除拾取列表的药品
  (bind _returnvalue (`|GetDataTableRow` "/Game/CJInventorySystem/Items/DrugList.DrugList" DrugName)
    (:`then`
      (for (_array_element _array_index) _containerslots
        (if (`KismetTextLibrary.EqualEqual_TextText` (`KismetTextLibrary.Conv_NameToText` (`.Name_11_4AC09FC14D48C480239495A1DC12C110` (break `/Game/CJInventorySystem/Blueprints/Inventory/DrugInfo` _returnvalue))) (`/Game/CJInventorySystem/UI/Blueprints/Inventory/ContainerSlot.NameValue` _array_element))
          (`KismetArrayLibrary.Array_Remove` _containerslots _array_index)
          (`self.RebuildContainer`)
          (if (<= (`KismetArrayLibrary.Array_Length` (`/Game/CJInventorySystem/UI/Blueprints/Inventory/Container.ContainerSlots` (`self.Container`))) 0)
            (`Widget.RemoveFromParent` (`self.Container`))
            (set `PlayerController.bShowMouseCursor` false (`GameplayStatics.GetPlayerController` 0))
            (set `self.IsShowMouseCursor` false)
            (set `self.IsCreateContainer` false)))))))